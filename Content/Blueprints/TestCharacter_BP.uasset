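; TestCharacter_BP is a test character that switches its morphing gun's effects between electric and flame bullet types.
; The construction script caches the WeaponActor child actor as a MorphingGunWeapon_BP reference.
; ElectricBullet and FlameBullet input presses set thunder-ball or fireball particle templates on both that weapon and a Projectile reference, which is not assigned in these graphs.
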(event `InputAction|ElectricBullet`
  (params (Key :type "Key Structure"))
  (:`Pressed`
    (`ParticleSystemComponent.SetTemplate` (`/MorphingGunPlugin/Weapon/Blueprints/MorphingGunWeapon_BP.ParticleSystem` (`self.Weapon`)) "/Game/FXVarietyPack/Particles/P_ky_thunderBall.P_ky_thunderBall")
    (`ParticleSystemComponent.SetTemplate` (`/MorphingGunPlugin/Projectile/Blueprints/MorphingGunProjectile_BP.ParticleSystem` (`self.Projectile`)) "/Game/FXVarietyPack/Particles/P_ky_thunderBall.P_ky_thunderBall")))

(event `InputAction|FlameBullet`
  (params (Key :type "Key Structure"))
  (:`Pressed`
    (`ParticleSystemComponent.SetTemplate` (`/MorphingGunPlugin/Weapon/Blueprints/MorphingGunWeapon_BP.ParticleSystem` (`self.Weapon`)) "/Game/FXVarietyPack/Particles/P_ky_fireBall.P_ky_fireBall")
    (`ParticleSystemComponent.SetTemplate` (`/MorphingGunPlugin/Projectile/Blueprints/MorphingGunProjectile_BP.ParticleSystem` (`self.Projectile`)) "/Game/FXVarietyPack/Particles/P_ky_fireBall.P_ky_fireBall")))

(fn `UserConstructionScript`
  (set `self.Weapon` (cast `/MorphingGunPlugin/Weapon/Blueprints/MorphingGunWeapon_BP` (`ChildActorComponent.ChildActor` (`self.WeaponActor`)) :!pure true)))